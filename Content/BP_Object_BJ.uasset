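; BP_Object_BJ is an actor that moves along world X at a configurable speed while showing a text label above it.
; On BeginPlay it casts its widget component to BP_TextWidget and sets the label from its TextAbove variable.
; Each Tick it rotates the widget to face the player camera and offsets the actor by Speed times delta time, without sweep.
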(event `self.ReceiveBeginPlay`
  (bind _asbp_text_widget (cast `/Game/BP_TextWidget` (`WidgetComponent.GetWidget` (`self.Widget`))))
  (set `self.As BP Text Widget` _asbp_text_widget)
  (`TextBlock.SetText` (`/Game/BP_TextWidget.text-above` (`self.As BP Text Widget`)) (`self.TextAbove`)))

(event `self.ReceiveTick`
  (params (DeltaSeconds :type "Float (single-precision)"))
  (`SceneComponent.K2_SetWorldRotation` (`self.Widget`) (`KismetMathLibrary.FindLookAtRotation` (`SceneComponent.K2_GetComponentLocation` (`self.Widget`)) (`SceneComponent.K2_GetComponentLocation` (`PlayerCameraManager.TransformComponent` (`GameplayStatics.GetPlayerCameraManager` 0)))) false false)
  (`self.K2_AddActorWorldOffset` (`KismetMathLibrary.MakeVector` (* DeltaSeconds (`self.Speed`)))))

(fn `UserConstructionScript`)